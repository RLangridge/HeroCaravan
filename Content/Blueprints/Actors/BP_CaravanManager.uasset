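; Manager actor that shows caravan avatars one at a time and cycles forward or backward through them.
; On BeginPlay it pre-spawns instances from PossibleCaravans at the root transform, up to a preload cap, and shows the first.
; Switching steps an index modulo the loaded array, walks the current avatar off or respawns an invalid target slot, then moves the new one to the billboard transform and walks it on stage.
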(event `self.ReceiveBeginPlay`
  (`self.Setup Transforms`)
  (bind _first_loaded_instance (`self.Pre-Load Caravans`))
  (bind _output_get (set `self.Active Caravan Instance` _first_loaded_instance))
  (`self.Show Caravan` _output_get))

(event `On Show Next Caravan`
  (params (`Is Getting Next?` :type Boolean))
  (bind _active_caravan_index (`self.Active Caravan Index`))
  (bind _index (`self.Get Next Index` (select `bool` `Is Getting Next?` :`false` -1 :`true` 1)))
  (if (`self.Is Caravan Loaded?` _index)
    (`/Game/Blueprints/Actors/BP_CaravanAvatar.On Walk Off Stage` (`self.Active Caravan Instance`))
    (else
      (`self.Load Caravan At Index` _active_caravan_index)))
  (bind _output_get (set `self.Active Caravan Instance` (`|GetArrayItem` (`self.Pre-Loaded Caravans`) _active_caravan_index)))
  (`self.Show Caravan` _output_get))

(fn `At Pre-load Capacity`
  (params (`Number Of Loaded Instances` :type Integer))
  (returns (`At Capacity` :type Boolean))
  (return (== `Number Of Loaded Instances` (`self.Number Of Instances To Pre-load`))))

(fn `Get Next Index`
  (params (Iterator :type Integer))
  (returns (Index :type Integer))
  (bind _output_get (set `self.Active Caravan Index` (mod (+ (`self.Active Caravan Index`) Iterator) (`KismetArrayLibrary.Array_Length` (`self.Pre-Loaded Caravans`)))))
  (return _output_get))

(fn `Is Caravan Loaded?`
  (params (`Caravan Index` :type Integer))
  (returns (`Is Loaded` :type Boolean))
  (return (`KismetSystemLibrary.IsValid` (`|GetArrayItem` (`self.Pre-Loaded Caravans`) `Caravan Index`))))

(fn `Load Caravan At Index`
  (params (Index :type Integer))
  (returns (`Loaded Caravan` :type "/Game/Blueprints/Actors/BP_CaravanAvatar Object Reference"))
  (bind _returnvalue (`|SpawnActorFromClass` (`|GetArrayItem` (`self.Possible Caravans`) Index) (`self.Caravan Spawn Transform`) "AlwaysSpawn" "OverrideRootScale" null null))
  (`KismetArrayLibrary.Array_Set` (`self.Pre-Loaded Caravans`) Index _returnvalue)
  (return _returnvalue))

(fn `Pre-Load Caravans`
  (returns (`First Loaded Instance` :type "/Game/Blueprints/Actors/BP_CaravanAvatar Object Reference"))
  (bind _pre_loaded_caravans (`self.Pre-Loaded Caravans`))
  (for (_array_element _array_index) (`self.Possible Caravans`)
    (if (`self.At Pre-load Capacity` _array_index)
      (break)
      (else
        (`self.Spawn In Caravan` _array_element))))
  (set `self.Number Of Instances Currently Loaded` (`KismetArrayLibrary.Array_Length` _pre_loaded_caravans))
  (return (`|GetArrayItem` _pre_loaded_caravans)))

(fn `Setup Transforms`
  (set `self.Show Caravan Transform` (`SceneComponent.K2_GetComponentToWorld` (`self.Show Off Caravan Transform Billboard`)))
  (set `self.Caravan Spawn Transform` (`SceneComponent.K2_GetComponentToWorld` (`self.DefaultSceneRoot`))))

(fn `Show Caravan`
  (params (`Caravan Instance` :type "/Game/Blueprints/Actors/BP_CaravanAvatar Object Reference"))
  (`/Game/Blueprints/Actors/BP_CaravanAvatar.On Walk On Stage` `Caravan Instance`)
  (`self.K2_SetActorTransform` `Caravan Instance` (`self.Show Caravan Transform`) false false))

(fn `Spawn In Caravan`
  (params (Class :type "Actor Object Reference"))
  (bind _returnvalue (`|SpawnActorFromClass` Class (`self.Caravan Spawn Transform`) "AlwaysSpawn" "OverrideRootScale" null null))
  (bind _asbp_caravan_avatar (cast `/Game/Blueprints/Actors/BP_CaravanAvatar` _returnvalue))
  (`KismetArrayLibrary.Array_Add` (`self.Pre-Loaded Caravans`) _asbp_caravan_avatar))

(fn `UserConstructionScript`)