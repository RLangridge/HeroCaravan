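; Pawn for the caravan setup flow, switching the player's view between caravan selection and a character view.
; It starts on CaravanCamera, then blends to CharacterCamera when a caravan is selected and back on return, using a configurable blend time and function.
; Next and previous events forward to CaravanManager to cycle the displayed caravan.
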(event `self.ReceiveBeginPlay`
  (`PlayerController.SetViewTargetWithBlend` (`GameplayStatics.GetPlayerController` 0) (`self.Caravan Camera`) 0.0 "VTBlend_Linear" 0.0 false))

(event `On Caravan Selected`
  (`PlayerController.SetViewTargetWithBlend` (`GameplayStatics.GetPlayerController` 0) (`self.Character Camera`) (`self.Camera Blend Time`) (`self.Blend Function`) 0.0 false))

(event `On Get Next Caravan`
  (`/Game/Blueprints/Actors/BP_CaravanManager.On Show Next Caravan` (`self.Caravan Manager`) true))

(event `On Get Previous Caravan`
  (`/Game/Blueprints/Actors/BP_CaravanManager.On Show Next Caravan` (`self.Caravan Manager`) false))

(event `On Return To Caravan Select`
  (`PlayerController.SetViewTargetWithBlend` (`GameplayStatics.GetPlayerController` 0) (`self.Caravan Camera`) (`self.Camera Blend Time`) (`self.Blend Function`) 0.0 false))

(fn `UserConstructionScript`)